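; BP_Pick_Bomb is a platformer pickup actor that changes the player's coin count by CoinsToAdd when touched.
; On BeginPlay it casts the first player controller to BP_ThirdPersonPlayerController and caches it.
; When the player character overlaps the Bomb component, it calls AddCoin on that controller, plays a placeholder sine-tone sound, spawns an emitter at its location and destroys itself.
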(event `self.bomb.OnComponentBeginOverlap`
  (params (OverlappedComponent :type "PrimitiveComponent Object Reference") (OtherActor :type "Actor Object Reference") (OtherComp :type "PrimitiveComponent Object Reference") (OtherBodyIndex :type Integer) (bFromSweep :type Boolean) (SweepResult :type "HitResult Structure (by ref)"))
  (if (== OtherActor (`GameplayStatics.GetPlayerCharacter` 0))
    (`/Game/ThirdPerson/Blueprints/BP_ThirdPersonPlayerController.Add Coin` (`self.Player Controller`) (`self.Coins To Add`))
    (`GameplayStatics.PlaySound2D` "/Engine/EngineSounds/1kSineTonePing.1kSineTonePing" 1.0 1.0 0.0 null null)
    (`GameplayStatics.SpawnEmitterAtLocation` null (`self.K2_GetActorLocation`))
    (`self.K2_DestroyActor`)))

(event `self.ReceiveBeginPlay`
  ; Creating reference to player controller
  (bind _asbp_third_person_player_controller (cast `/Game/ThirdPerson/Blueprints/BP_ThirdPersonPlayerController` (`GameplayStatics.GetPlayerController` 0)))
  (set `self.Player Controller` _asbp_third_person_player_controller))

(fn `UserConstructionScript`)