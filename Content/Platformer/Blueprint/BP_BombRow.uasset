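; BP_BombRow is an actor that groups child bomb actors into a row for the platformer's bomb mechanic.
; Its Fuze event lights the first child bomb through the BPI_Bombs interface.
; Tick polls the child actor list, and once it is empty asks the level's BP_BombController to light a random bomb, then destroys the row.
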(event `/Game/Platformer/Interfaces/BPI_Bombs.Fuze`
  ;[0.15 0.06038 0.05802 0.5] Light the first bomb
  (bind _asbpi_bombs (cast `/Game/Platformer/Interfaces/BPI_Bombs` (`|GetArrayItem` (`self.GetAllChildActors` false))))
  (`/Game/Platformer/Interfaces/BPI_Bombs.Fuze` _asbpi_bombs))

(event `self.ReceiveTick`
  (params (DeltaSeconds :type "Float (single-precision)"))
  ;[0.06319 0.07729 0.15 0.5] Destroy when no bombs
  (if (== (`KismetArrayLibrary.Array_Length` (`self.GetAllChildActors` false)) 0)
    (bind _returnvalue (`GameplayStatics.GetActorOfClass` "/Game/Platformer/Blueprint/BP_BombController.BP_BombController_C"))
    (`/Game/Platformer/Blueprint/BP_BombController.LightRandomBomb` _returnvalue)
    (`self.K2_DestroyActor`)))

(fn `UserConstructionScript`)