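; BP_Bomb is a collectible bomb that awards coins through the player controller when the player overlaps it.
; Pickup plays a sound and spawns an emitter, then destroys the bomb a frame later.
; A lit bomb first sends a Fuze message to bombs overlapping its NearCollider.
; Fuze marks a bomb as lit and swaps its sphere to the lit material, so lighting passes along as bombs are collected.
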(event `self.bomb.OnComponentBeginOverlap`
  (params (OverlappedComponent :type "PrimitiveComponent Object Reference") (OtherActor :type "Actor Object Reference") (OtherComp :type "PrimitiveComponent Object Reference") (OtherBodyIndex :type Integer) (bFromSweep :type Boolean) (SweepResult :type "HitResult Structure (by ref)"))
  ;[0.02749 0.04614 0.15 0.5] Pickup
  (if (== OtherActor (`GameplayStatics.GetPlayerCharacter` 0))
    (`/Game/ThirdPerson/Blueprints/BP_ThirdPersonPlayerController.Add Coin` (`self.Player Controller`) (`self.Coins To Add`))
    (`GameplayStatics.PlaySound2D` "/Engine/EngineSounds/1kSineTonePing.1kSineTonePing" 1.0 1.0 0.0 null null)
    (`GameplayStatics.SpawnEmitterAtLocation` null (`self.K2_GetActorLocation`))
    (if (`self.IsLit`)
      (for _array_element (`PrimitiveComponent.GetOverlappingActors` (`self.NearCollider`) "BP_Bomb_C")
        (message `/Game/Platformer/Interfaces/BPI_Bombs.Fuze` _array_element)
        (`KismetSystemLibrary.DelayUntilNextFrame` :!label _label)
        (`self.K2_DestroyActor`))
      (else
        (goto _label)))))

(event `/Game/Platformer/Interfaces/BPI_Bombs.Fuze`
  (set `self.IsLit` true)
  (`PrimitiveComponent.SetMaterial` (`self.Sphere`) 0 "/Game/Platformer/Materials/M_BombLit.M_BombLit"))

(event `self.ReceiveBeginPlay`
  ; Creating reference to player controller
  (bind _asbp_third_person_player_controller (cast `/Game/ThirdPerson/Blueprints/BP_ThirdPersonPlayerController` (`GameplayStatics.GetPlayerController` 0)))
  (set `self.Player Controller` _asbp_third_person_player_controller))

(fn `UserConstructionScript`)