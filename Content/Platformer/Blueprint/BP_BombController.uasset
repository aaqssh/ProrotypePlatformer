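; BP_BombController starts the platformer's bomb sequence and runs its countdown timer.
; On BeginPlay it waits one tick, picks a random BP_BombRow in the level and calls FuzeMessage on it to light the first bomb.
; Tick counts Timer down from its default and stores a truncated copy in TimerRounded.
; Expiry only prints a placeholder "explosion" string, repeated every frame from zero onward.
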(event `LightRandomBomb`
  ;[1 0.07187 0.07187 0.5] Light first bomb
  (`KismetSystemLibrary.DelayUntilNextTick`)
  (bind _outactors (`GameplayStatics.GetAllActorsOfClass` "/Game/Platformer/Blueprint/BP_BombRow.BP_BombRow_C"))
  (message `/Game/Platformer/Interfaces/BPI_Bombs.Fuze` (`KismetArrayLibrary.Array_Random` _outactors)))

(event `self.ReceiveTick`
  (params (DeltaSeconds :type "Float (single-precision)"))
  (bind _output_get (set `self.Timer` (- (`self.Timer`) DeltaSeconds)))
  (set `self.TimerRounded` (`KismetMathLibrary.FTrunc` _output_get))
  (if (<= _output_get 0.0)
    (`KismetSystemLibrary.PrintString` "explosion")))

(event `self.ReceiveBeginPlay`
  (`self.LightRandomBomb`)
  (set `self.Timer` (`self.TimerDefaultValue`)))

(fn `UserConstructionScript`)