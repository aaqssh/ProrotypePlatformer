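; Bomb game controller that runs the countdown and decides victory or game over.
; On start it lights a random BP_BombRow fuze, then Tick drains the timer, which AddTime extends.
; At zero, Loss damages the player and resets the timer, or on last health explodes the sphinx and all bombs in staggered sequence before loading LV_GameOver.
; NoBombs loads LV_Victory once no BP_BombSingle remains.
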(event `LightRandomBomb`
  ;[1 0.07187 0.07187 0.5] Light Random bomb on startup
  (`KismetSystemLibrary.DelayUntilNextTick`)
  (bind _outactors (`GameplayStatics.GetAllActorsOfClass` "/Game/BombJackContent/Blueprint/Bomb/BP_BombRow.BP_BombRow_C"))
  (message `/Game/BombJackContent/Blueprint/Interfaces/BPI_Bombs.Fuze` (`KismetArrayLibrary.Array_Random` _outactors)))

(event `Loss`
  (bind _bombexplosion (`self.BombExplosion`))
  ;[0.04259 0.15 0.03797 0.5] Check Loss status
  (bind _returnvalue (`GameplayStatics.GetActorOfClass` "/Game/BombJackContent/Blueprint/Player/BP_BombJackThirdPerson.BP_BombJackThirdPerson_C"))
  (if (> (`/Game/BombJackContent/Blueprint/Player/BP_BombJackThirdPerson.CurrentHealth` _returnvalue) 1.0)
    (`GameplayStatics.ApplyDamage` _returnvalue 1.0)
    (set `self.Timer` (`self.TimerAddAmount`))
    (else
      (`ActorComponent.Activate` (`self.LossExplosion`) false)
      (`AudioComponent.AdjustVolume` _bombexplosion 0.0 100.0 "Linear")
      (`AudioComponent.Play` _bombexplosion 0.0)
      (`SceneComponent.ToggleVisibility` (`self.SphinxLod0_3`) false)
      (`SceneComponent.ToggleVisibility` (`self.ExplodedSphinxLod0`) false)
      (set `self.Active` false)
      (`self.ExplodeAllBombs`)
      (`KismetSystemLibrary.Delay` 5.0)
      (`GameplayStatics.OpenLevel` "LV_GameOver"))))

(event `self.ReceiveTick`
  (params (DeltaSeconds :type "Float (single-precision)"))
  ;[0.04259 0.15 0.03797 0.5] Check Loss status
  ;;[0.08694 0.5041 0.6858 0.5] Is the timer 0?
  (if (`self.Active`)
    (bind _output_get (set `self.Timer` (- (`self.Timer`) DeltaSeconds)))
    (set `self.TimerRounded` (`KismetMathLibrary.FTrunc` _output_get))
    (if (<= _output_get 0.0)
      (`KismetSystemLibrary.PrintString` "explosion")
      (`GameplayStatics.GetAllActorsOfClass` "/Game/BombJackContent/Blueprint/Bomb/BP_BombSingle.BP_BombSingle_C")
      (`self.Loss`))))

(event `NoBombs`
  ;[0 0.1839 1 0.5] Did you win? (Are all the bombs picked up)
  (bind _returnvalue (`GameplayStatics.GetActorOfClass` "/Game/BombJackContent/Blueprint/Bomb/BP_BombSingle.BP_BombSingle_C"))
  (`/Engine/EditorBlueprintResources/StandardMacros.IsValid` _returnvalue
    (:`Is Not Valid`
      (`KismetSystemLibrary.PrintString` "END")
      (`KismetSystemLibrary.Delay` 2.0)
      (`GameplayStatics.OpenLevel` "LV_Victory"))))

(event `ExplodeAllBombs`
  ;[0.04259 0.15 0.03797 0.5] Check Loss status
  (bind _outactors (`GameplayStatics.GetAllActorsOfClass` "/Game/BombJackContent/Blueprint/Bomb/BP_BombSingle.BP_BombSingle_C"))
  (for (_array_element _array_index) _outactors
    (`/Game/BombJackContent/Blueprint/Bomb/BP_BombSingle.Explode` _array_element (* _array_index 0.2))))

(event `self.ReceiveBeginPlay`
  ;[0.9823 0.7981 0 0.5] Light a bomb start of game
  (`AudioComponent.AdjustVolume` (`self.BombExplosion`) 0.0 -100.0 "Linear")
  (`self.LightRandomBomb`)
  (set `self.Timer` (`self.TimerDefaultValue`)))

(event `AddTime`
  ;[0.9913 0 0.9188 0.5] Add Time Function
  (set `self.Timer` (+ (`self.Timer`) (`self.TimerAddAmount`))))

(fn `UserConstructionScript`)