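; A collectible Bomb Jack-style bomb that awards coins when the player character overlaps it, then destroys itself a tick later.
; Pickup plays a sound and emitter; if lit, it also sends a fuse message to overlapping BP_BombSingle actors in its NearCollider.
; Its Fuze event lights it, showing smoke, swapping to the lit material and resetting the BP_BombController timer.
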(event `self.bomb.OnComponentBeginOverlap`
  (params (OverlappedComponent :type "PrimitiveComponent Object Reference") (OtherActor :type "Actor Object Reference") (OtherComp :type "PrimitiveComponent Object Reference") (OtherBodyIndex :type Integer) (bFromSweep :type Boolean) (SweepResult :type "HitResult Structure (by ref)"))
  ;[0.02749 0.04614 0.15 0.5] Pickup
  (if (== OtherActor (`GameplayStatics.GetPlayerCharacter` 0))
    (`/Game/BombJackContent/Blueprint/Player/BP_BombJackController.Add Coin` (`self.Player Controller`) (`self.Coins To Add`))
    (`GameplayStatics.PlaySound2D` "/Engine/EngineSounds/1kSineTonePing.1kSineTonePing" 1.0 1.0 0.0 null null)
    (`GameplayStatics.SpawnEmitterAtLocation` null (`self.K2_GetActorLocation`))
    (if (`self.IsLit`)
      (for _array_element (`PrimitiveComponent.GetOverlappingActors` (`self.NearCollider`) "/Game/BombJackContent/Blueprint/Bomb/BP_BombSingle.BP_BombSingle_C")
        (message `/Game/BombJackContent/Blueprint/Interfaces/BPI_Bombs.Fuze` _array_element)
        (`KismetSystemLibrary.DelayUntilNextTick` :!label _label)
        (`self.K2_DestroyActor`))
      (else
        (goto _label)))))

(event `self.Fuze`
  ;[0.5865 0.2605 0.5159 0.5] Light Bomb
  (`SceneComponent.SetVisibility` (`self.Smoke`) true false)
  (set `self.IsLit` true)
  (`PrimitiveComponent.SetMaterial` (`self.Sphere`) 0 "/Game/BombJackContent/Materials/M_BombLit.M_BombLit")
  (bind _returnvalue (`GameplayStatics.GetActorOfClass` "/Game/BombJackContent/Blueprint/Bomb/BP_BombController.BP_BombController_C"))
  (set `/Game/BombJackContent/Blueprint/Bomb/BP_BombController.Timer` (`/Game/BombJackContent/Blueprint/Bomb/BP_BombController.TimerDefaultValue` _returnvalue) _returnvalue))

(event `self.ReceiveBeginPlay`
  ; Creating reference to player controller
  (bind _asbp_bomb_jack_controller (cast `/Game/BombJackContent/Blueprint/Player/BP_BombJackController` (`GameplayStatics.GetPlayerController` 0)))
  (set `self.Player Controller` _asbp_bomb_jack_controller))

(fn `UserConstructionScript`)