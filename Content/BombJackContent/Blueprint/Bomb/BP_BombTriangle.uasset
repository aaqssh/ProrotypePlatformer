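; BP_BombTriangle is a group of child-actor bombs that acts as one row managed by BP_BombController.
; Fuze marks the row lit, lights the first child through BPI_Bombs, and debug-prints whether the row is far right or left of the player on X.
; Tick polls for remaining children; when none are left it has the controller light a random bomb if this row was lit, calls NoBombs, then destroys itself.
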(event `self.Fuze`
  (bind _returnvalue_x (`KismetMathLibrary.BreakVector` (`SceneComponent.K2_GetComponentLocation` (`self.DefaultSceneRoot`))))
  ;[0.15 0.06038 0.05802 0.5] On Fuze Event
  ;; Light first Bomb
  (`|ExecutionSequence`
    (:`then_0`
      (set `self.IsLitRow` true)
      (bind _asbpi_bombs (cast `/Game/BombJackContent/Blueprint/Interfaces/BPI_Bombs` (`|GetArrayItem` (`self.GetAllChildActors` false))))
      (`/Game/BombJackContent/Blueprint/Interfaces/BPI_Bombs.Fuze` _asbpi_bombs))
    (:`then_1`
      ;; Get arrow from player to bomb
      (bind _returnvalue (`GameplayStatics.GetActorOfClass` "/Game/BombJackContent/Blueprint/Player/BP_BombJackThirdPerson.BP_BombJackThirdPerson_C"))
      (bind _returnvalue_x_2 (`KismetMathLibrary.BreakVector` (`SceneComponent.K2_GetComponentLocation` (`Actor.RootComponent` _returnvalue))))
      (bind _returnvalue_2 (- _returnvalue_x _returnvalue_x_2))
      (if (> _returnvalue_2 1000.0)
        (`KismetSystemLibrary.PrintString` "Right")
        (elif (< _returnvalue_2 -1000.0)
          (`KismetSystemLibrary.PrintString` "Left"))))))

(event `self.ReceiveTick`
  (params (DeltaSeconds :type "Float (single-precision)"))
  ;[0.06319 0.07729 0.15 0.5] Destroy when no bombs
  (if (== (`KismetArrayLibrary.Array_Length` (`self.GetAllChildActors` false)) 0)
    (bind _returnvalue (`GameplayStatics.GetActorOfClass` "/Game/BombJackContent/Blueprint/Bomb/BP_BombController.BP_BombController_C"))
    (if (`self.IsLitRow`)
      (`/Game/BombJackContent/Blueprint/Bomb/BP_BombController.LightRandomBomb` _returnvalue))
    (bind _returnvalue_2 (`GameplayStatics.GetActorOfClass` "/Game/BombJackContent/Blueprint/Bomb/BP_BombController.BP_BombController_C"))
    (`/Game/BombJackContent/Blueprint/Bomb/BP_BombController.NoBombs` _returnvalue_2)
    (`self.K2_DestroyActor`)))

(fn `UserConstructionScript`)