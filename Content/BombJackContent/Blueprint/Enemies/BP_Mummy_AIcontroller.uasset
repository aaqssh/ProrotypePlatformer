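; BP_Mummy_AIcontroller is the AI controller for the Mummy enemy.
; On BeginPlay it runs the Mummy_BT behavior tree and casts its pawn to BP_Mummy.
; It seeds the blackboard with two patrol endpoints: StartPatrol at the pawn's location, and PatrolLocation as that location plus the Mummy's MummyPatrolPoint, treated as a local offset.
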(event `self.ReceiveBeginPlay`
  (bind _returnvalue (`self.K2_GetPawn`))
  (bind _returnvalue_2 (`self.K2_GetActorLocation` _returnvalue))
  (`self.RunBehaviorTree` "/Game/BombJackContent/Blueprint/Enemies/Mummy_BT.Mummy_BT")
  (bind _asbp_mummy (cast `/Game/BombJackContent/Blueprint/Enemies/BP_Mummy` _returnvalue))
  (`BlackboardComponent.SetValueAsVector` (`self.Blackboard`) "PatrolLocation" (+ (`/Game/BombJackContent/Blueprint/Enemies/BP_Mummy.MummyPatrolPoint` _asbp_mummy) _returnvalue_2 (0.0 0.0 0.0)))
  (`BlackboardComponent.SetValueAsVector` (`self.Blackboard`) "StartPatrol" _returnvalue_2))

(fn `UserConstructionScript`)